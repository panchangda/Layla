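; GA_SpeedUp is a Gameplay Ability that temporarily raises the Layla character's walk speed.
; After committing, it caches MaxWalkSpeed, scales it by SpeedUpMultiplier, applies GE_SpeedUp and adds a gameplay cue, or cancels if the commit fails.
; The effect's lifetime drives the ability: its removal or an invalid handle ends it.
; OnEndAbility restores the cached speed, and the cue is removed automatically.
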(event Ability|EventActivateAbility
  (bind _returnvalue (Class|LaylaGameplayAbility|GetLaylaCharacterfromActorInfo))
  (bind _charactermovement (Variables|/Script/Engine.Character|GetCharacterMovement _returnvalue))
  ;[1 1 1] Commit:Test Cooldown
  (bind _returnvalue_2 (Ability|CommitAbility))
  (if _returnvalue_2
    (bind _output_get (Variables|Default|SetDefault%20Max%20Speed (Variables|/Script/Engine.CharacterMovementComponent|GetMaxWalkSpeed _charactermovement)))
    (Variables|/Script/Engine.CharacterMovementComponent|SetMaxWalkSpeed _charactermovement (* _output_get (Variables|Default|GetSpeed%20Up%20Multiplier)))
    (bind _returnvalue_3 (Ability|ApplyGameplayEffectToOwner "/Game/Characters/Heroes/Abilities/SpeedUp/GE_SpeedUp.GE_SpeedUp_C"))
    (Variables|Default|SetGE%20Speed%20Up _returnvalue_3)
    (GameplayCue|AddGameplayCue :GameplayCueTag "(TagName=\"GameplayCue.Hero.SpeedUp\")")
    (|WaitforGameplayEffectRemoved (Variables|Default|GetGE%20Speed%20Up)
      (:OnRemoved
        _)
      (:InvalidHandle
        _))
    (Ability|EndAbility)
    (else
      (Ability|CancelAbility))))

(event Ability|EventOnEndAbility
  (params (bWasCancelled :type Boolean))
  (Variables|/Script/Engine.CharacterMovementComponent|SetMaxWalkSpeed (Variables|/Script/Engine.Character|GetCharacterMovement (Class|LaylaGameplayAbility|GetLaylaCharacterfromActorInfo)) (Variables|Default|GetDefault%20Max%20Speed)))