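; Main menu player controller that shows the menu UI and a preview of the player's hero.
; On BeginPlay, the local controller adds the W_MainMenu widget, enables the mouse cursor and calls SpawnHeroActor.
; That event destroys any previous hero actor and spawns the character class stored in LaylaGameInstance's Hero data at the transform of the first Pawn found, so repeat calls replace the displayed hero.
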(event Custom|SpawnHeroActor
  (bind _aslayla_game_instance (Utilities|Casting|CastToLaylaGameInstance (Game|GetGameInstance)))
  (Utilities|IsValid (Variables|Default|GetLast%20Player%20Class)
    (:Is%20Valid
      (Actor|DestroyActor (Variables|Default|GetLast%20Player%20Class)))
    (:Is%20Not%20Valid
      _))
  (bind _asactor (Utilities|Casting|CastToActorClass (.CharacterBP (Utilities|Struct|BreakLaylaHeroStruct (Variables|/Script/Layla.LaylaGameInstance|GetHero _aslayla_game_instance)))))
  (bind _returnvalue (Actor|GetActorOfClass "/Script/Engine.Pawn"))
  (bind _returnvalue_2 (Game|SpawnActorfromClass _asactor (Transformation|GetActorTransform _returnvalue) "Undefined" "MultiplyWithRoot" 0 0))
  (Variables|Default|SetLast%20Player%20Class _returnvalue_2)
  (Networking|SetReplicates false))

(event EventBeginPlay
  (if (Pawn|IsLocalPlayerController)
    (bind _returnvalue (UserInterface|CreateWidget "/Game/UI/MainMenu/W_MainMenu.W_MainMenu_C" self))
    (UserInterface|Viewport|AddtoViewport _returnvalue 0)
    (Variables|Default|SetbShowMouseCursor true)
    (CallFunction|SpawnHeroActor)))

(event EventTick
  (params (DeltaSeconds :type Float%20%28single-precision%29)))

(fn ConstructionScript)